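; GoldPickup is a gold pickup Blueprint that animates itself by spinning and bobbing; it contains no collection logic.
; Each Tick adds a yaw step from StartingRotation plus a constant to the root component.
; A wrapping angle counter feeds a degree sine, which is added as an unswept relative Z offset for the bob.
; Both motions use per-frame steps without delta time, so their speed follows frame rate.
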(event EventTick
  (params (DeltaSeconds :type Float%20%28single-precision%29))
  (bind _self self)
  (bind _returnvalue (VehicleSound|GetRootComponent _self))
  (Transformation|AddRelativeRotation _returnvalue (Math|Rotator|MakeRotator 0.0 0.0 (+ (Variables|Default|GetStartingRotation) 5.0)) false false)
  (if (>= (Variables|Default|GetZMovVal) 355.0)
    (Variables|Default|SetZMovVal 0.0))
  (bind _output_get (Variables|Default|SetZMovVal (+ (Variables|Default|GetZMovVal) 8.0)))
  (bind _output_get_2 (Variables|Default|SetStaringMovement (Math|Vector|MakeVector 0.0 0.0 (Math|Trig|Sin(Degrees) _output_get))))
  (Transformation|AddRelativeLocation _returnvalue _output_get_2 false false))

(event EventBeginPlay
  (Variables|Default|SetStaringMovement "0, 0, 0")
  (Variables|Default|SetZMovVal 0.0))

(fn ConstructionScript)