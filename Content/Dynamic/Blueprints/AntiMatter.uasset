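; AntiMatter is a pickup actor that awards 1000 points when a JimCharacter overlaps it.
; It caches the JimGame game mode on BeginPlay, then uses it to raise the score and play the PickupSuccess effect.
; A DoOnce limits the reward to a single trigger, which also sets an Active flag and destroys the actor after a short delay.
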(event EventBeginPlay
  ;[1 1 1] Game setup
  (bind _asjim_game (Utilities|Casting|CastToJimGame (Game|GetGameMode)))
  (Variables|Default|SetJimGame _asjim_game))

(event Collision|EventActorBeginOverlap
  (params (OtherActor :type Actor%20Object%20Reference))
  (bind _jimgame (Variables|Default|GetJimGame))
  ;[1 1 1] Collision handling
  (Utilities|Casting|CastToJimCharacter OtherActor)
  (Utilities|FlowControl|DoOnce false
    (:Completed
      (Variables|Default|Setactive true)
      (Variables|/Game/Dynamic/Blueprints/JimGame.JimGame_C|SetScore _jimgame (+ (Variables|/Game/Dynamic/Blueprints/JimGame.JimGame_C|GetScore _jimgame) 1000))
      (Audio|Components|Audio|Play (Variables|/Game/Dynamic/Blueprints/JimGame.JimGame_C|GetPickupSuccess _jimgame) 0.0)
      (Utilities|FlowControl|Delay 0.1)
      (Actor|DestroyActor))))

(fn ConstructionScript)