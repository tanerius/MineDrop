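; JimFire is a fire hazard that kills JimCharacter on touch and can be put out by clicking it repeatedly for points.
; On overlap it freezes player and level-item movement through JimGame, plays the death sound and flags the anim Blueprint dead.
; After a short delay it destroys the character and calls PlayerDies.
; Click releases count while the player can move, until the fire awards score, plays a sound and destroys itself.
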(event EventBeginPlay
  ;[1 1 1] Game setup
  (bind _asjim_game (Utilities|Casting|CastToJimGame (Game|GetGameMode)))
  (Variables|Default|SetJimGame _asjim_game))

(event Collision|EventActorBeginOverlap
  (params (OtherActor :type Actor%20Object%20Reference))
  (bind _jimgame (Variables|Default|GetJimGame))
  ;[1 1 1] Touch death by fire
  (bind _asjim_character (Utilities|Casting|CastToJimCharacter OtherActor))
  (Variables|Default|SetJimCharacter _asjim_character)
  (Variables|Default|Setactive false)
  (Variables|/Game/Dynamic/Blueprints/JimGame.JimGame_C|SetCanMovePlayer _jimgame false)
  (Variables|/Game/Dynamic/Blueprints/JimGame.JimGame_C|SetCanMoveLevelItems _jimgame false)
  (Audio|Components|Audio|Play (Variables|/Game/Dynamic/Blueprints/JimGame.JimGame_C|GetDeathSound (Variables|Default|GetJimGame)) 0.0)
  (bind _asbp_jim_anims (Utilities|Casting|CastToBP_Jim_Anims (Components|SkeletalMesh|GetAnimInstance (Variables|/Script/Engine.Character|GetMesh (Variables|Default|GetJimCharacter)))))
  (Variables|Default|SetJimAnims _asbp_jim_anims)
  (Variables|/Game/Dynamic/JimCharacter/BP_Jim_Anims.BP_Jim_Anims_C|SetIsNotDead? (Variables|Default|GetJimAnims) false)
  (Variables|/Game/Dynamic/JimCharacter/BP_Jim_Anims.BP_Jim_Anims_C|SetIsDead (Variables|Default|GetJimAnims) true)
  (Utilities|FlowControl|Delay 0.8)
  (Actor|DestroyActor (Variables|Default|GetJimCharacter))
  (Default|PlayerDies (Variables|Default|GetJimGame)))

(event EventActorOnReleased
  (params (ButtonReleased :type Key%20Structure :default "AnyKey"))
  (bind _jimgame (Variables|Default|GetJimGame))
  ;[1 1 1] Putting out fires - score updates
  (if (Variables|/Game/Dynamic/Blueprints/JimGame.JimGame_C|GetCanMovePlayer (Variables|Default|GetJimGame))
    (Utilities|FlowControl|Delay 0.03)
    (if (== (Variables|Default|GetClickedOn) 2)
      (Variables|/Game/Dynamic/Blueprints/JimGame.JimGame_C|SetScore _jimgame (+ (Variables|/Game/Dynamic/Blueprints/JimGame.JimGame_C|GetScore _jimgame) 50))
      (Audio|Components|Audio|Play (Variables|/Game/Dynamic/Blueprints/JimGame.JimGame_C|GetExtFire _jimgame) 0.0)
      (Actor|DestroyActor)
      (else
        (Variables|Default|SetClickedOn (+ (Variables|Default|GetClickedOn) 1))))))

(fn ConstructionScript)