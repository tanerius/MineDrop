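; One of two swapping platform sets that form an endlessly descending, randomized level in JimGame.
; Builds six rows of six tiles by toggling visibility and collision: tiles below gaps are forced on, others randomized under a five-tile cap.
; Gaps carry row to row, seeded from TopPlatformSet on the first set's first run, otherwise from its partner.
; When regenerated, it moves down and arms a JimCharacter overlap that triggers the partner's rebuild.
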(event OnComponentBeginOverlap(Group5)
  (params (OverlappedComponent :type Primitive%20Component%20Object%20Reference) (OtherActor :type Actor%20Object%20Reference) (OtherComp :type Primitive%20Component%20Object%20Reference) (OtherBodyIndex :type Integer) (bFromSweep :type Boolean) (SweepResult :type Hit%20Result%20Structure%20%28by%20ref%29))
  (bind _otherswappingplatform (Variables|Default|GetOtherSwappingPlatform))
  ;[1 1 1] Generate a new platform level when 5th level tiles are overlapped
  (if (not (Variables|Default|GetWaitSuccess))
    (Variables|Default|SetWaitSuccess true)
    (Utilities|Casting|CastToJimCharacter OtherActor
      (:then
        (Utilities|FlowControl|DoOnce false
          (:Completed
            (if (Variables|Default|GetIsFirstRun)
              (Variables|Default|SetIsFirstRun false)
              (CallFunction|CreateSelf _otherswappingplatform)
              (else
                (CallFunction|RecreateandMove _otherswappingplatform))))))
      (:CastFailed
        (Variables|Default|SetWaitSuccess false)))))

(event Custom|CreateSelf
  (bind _1_2 (Variables|PlatformMeshes|Get1.2))
  (bind _1_3 (Variables|PlatformMeshes|Get1.3))
  (bind _1_4 (Variables|PlatformMeshes|Get1.4))
  (bind _1_5 (Variables|PlatformMeshes|Get1.5))
  (bind _1_6 (Variables|PlatformMeshes|Get1.6))
  (bind _1_1 (Variables|PlatformMeshes|Get1.1))
  (bind _array (Utilities|Array|MakeArray _1_1 _1_2 _1_3 _1_4 _1_5 _1_6))
  ;[1 1 1] Creation sequence
  (Utilities|FlowControl|Sequence
    (:then_0
      ;[1 1 1] Get Gaps from platform set above this one
      (if (and (Variables|Default|GetIsFirstMovingPlatform) (Variables|Default|GetIsFirstRun))
        (Variables|Default|SetGapsLocal (Variables|/Game/Dynamic/Blueprints/TopPlatformSet.TopPlatformSet_C|GetGaps (Variables|Default|GetTopPlatformSet)))
        (else
          (Variables|Default|SetGapsLocal (Variables|UpperPlatformSet_C|GetGapsLocal (Variables|Default|GetOtherSwappingPlatform))))))
    (:then_1
      ;[1 1 1] Generate first level
      ;;[1 1 1] Step 1: Disable all tiles
      (for _array_element _array
        (CallFunction|ToggleFloorTile false false _array_element)
        (Variables|Default|SetPlatformsVisible 0))
      ;;[1 1 1] Step 2: Set tiles directly underneath previous gaps (game rule)
      (for _array_element_2 _array
        (for _array_element_3 (Variables|Default|GetGapsLocal)
          (if (and (Variables|Default|GetIsFirstMovingPlatform) (Variables|Default|GetIsFirstRun))
            (if (== _array_element_3 (+ (Math|Conversions|ToFloat(Integer) (Utilities|String|ToString(Object) _array_element_2)) 2.0))
              (CallFunction|ToggleFloorTile true true _array_element_2 :!label _label))
            (elif (== _array_element_3 (+ (Math|Conversions|ToFloat(Integer) (Utilities|String|ToString(Object) _array_element_2)) 5.0))
              (goto _label)))))
      (Utilities|Array|Clear (Variables|Default|GetGapsLocal))
      ;;[1 1 1] Step 3: Randomize visibility of unset tiles
      (for _array_element_4 _array
        (if (not (Rendering|IsVisible _array_element_4))
          (if (< (Variables|Default|GetPlatformsVisible) 5)
            (bind _randomval (CallFunction|RandomToggle))
            (bind _hasenabled (CallFunction|ToggleFloorTile _randomval true _array_element_4))
            (if (not _hasenabled)
              (Utilities|Array|Add (Variables|Default|GetGapsLocal) (Math|Conversions|ToFloat(Integer) (Utilities|String|ToString(Object) _array_element_4)) :!label _label_2))
            (else
              (goto _label_2))))))
    (:then_2
      ;[1 1 1] Generate remaining platform levels
      (CallFunction|GeneratePlatforms (Utilities|Array|MakeArray (Variables|PlatformMeshes|Get2.1) (Variables|PlatformMeshes|Get2.2) (Variables|PlatformMeshes|Get2.3) (Variables|PlatformMeshes|Get2.4) (Variables|PlatformMeshes|Get2.5) (Variables|PlatformMeshes|Get2.6)))
      (CallFunction|GeneratePlatforms (Utilities|Array|MakeArray (Variables|PlatformMeshes|Get3.1) (Variables|PlatformMeshes|Get3.2) (Variables|PlatformMeshes|Get3.3) (Variables|PlatformMeshes|Get3.4) (Variables|PlatformMeshes|Get3.5) (Variables|PlatformMeshes|Get3.6)))
      (CallFunction|GeneratePlatforms (Utilities|Array|MakeArray (Variables|Default|Get4.1) (Variables|Default|Get4.2) (Variables|Default|Get4.3) (Variables|Default|Get4.4) (Variables|Default|Get4.5) (Variables|Default|Get4.6)))
      (CallFunction|GeneratePlatforms (Utilities|Array|MakeArray (Variables|Default|Get5.1) (Variables|Default|Get5.2) (Variables|Default|Get5.3) (Variables|Default|Get5.4) (Variables|Default|Get5.5) (Variables|Default|Get5.6)))
      (CallFunction|GeneratePlatforms (Utilities|Array|MakeArray (Variables|Default|Get6.1) (Variables|Default|Get6.2) (Variables|Default|Get6.3) (Variables|Default|Get6.4) (Variables|Default|Get6.5) (Variables|Default|Get6.6))))
    (:then_3
      (Variables|Default|SetWaitSuccess false))))

(event Custom|RecreateAndMove
  (bind _otherswappingplatform (Variables|Default|GetOtherSwappingPlatform))
  ;[1 1 1] Recreate and move sequence
  (Utilities|FlowControl|Sequence
    (:then_0
      (CallFunction|CreateSelf))
    (:then_1
      ;[1 1 1] Move platform
      (Transformation|SetActorLocation (+ (Transformation|GetActorLocation) "0, 0,-2880.000000") false false)
      ;[1 1 1] Generate a new platform level when 5th level tiles are overlapped
      (Utilities|FlowControl|DoOnce false) ; enters at Reset
    )
    (:then_2
      (Variables|Default|SetWaitSuccess false))))

(event EventBeginPlay
  (bind _asjim_game (Utilities|Casting|CastToJimGame (Game|GetGameMode)))
  (Variables|Default|SetGameStore _asjim_game)
  (Utilities|FlowControl|Sequence
    (:then_0
      ;[1 1 1] Set reference to top platform
      (bind _outactors (Actor|GetAllActorsOfClass "/Game/Dynamic/Blueprints/TopPlatformSet.TopPlatformSet_C"))
      (Variables|Default|SetTopPlatformSet (Utilities|Array|Get(acopy) _outactors)))
    (:then_1
      ;[1 1 1] Set reference to other swapping platform
      (bind _outactors_2 (Actor|GetAllActorsOfClass "UpperPlatformSet_C"))
      (for _array_element _outactors_2
        (if (not (Utilities|Enum|Equal(Enum) (Utilities|GetDisplayName _array_element) (Utilities|GetDisplayName self)))
          (Variables|Default|SetOtherSwappingPlatform _array_element))))
    (:then_2
      ;[1 1 1] Set up timing control vars
      (if (Variables|Default|GetIsFirstMovingPlatform)
        (Variables|Default|SetIsFirstRun true)
        (Utilities|Array|SetArrayElem (Variables|/Game/Dynamic/Blueprints/JimGame.JimGame_C|GetSetupVars (Variables|Default|GetGameStore)) 1 true)
        (else
          (Utilities|Array|SetArrayElem (Variables|/Game/Dynamic/Blueprints/JimGame.JimGame_C|GetSetupVars (Variables|Default|GetGameStore)) 2 true))))
    (:then_3
      (Variables|Default|SetWaitSuccess false))))

(fn ConstructionScript)

(fn GeneratePlatforms
  (params (PlatformsArry :type Array%20of%20Static%20Mesh%20Component%20Object%20References))
  ;[1 1 1] Step 1: Set all tiles to inviz
  (Variables|Default|SetPlatformsVisible 0)
  (for _array_element PlatformsArry
    (CallFunction|ToggleFloorTile false false _array_element))
  ;[1 1 1] Step 2: Enable tiles below inviz tiles (game rule)
  (for _array_element_2 PlatformsArry
    (for _array_element_3 (Variables|Default|GetGapsLocal)
      (if (== (+ _array_element_3 1.0) (Math|Conversions|ToFloat(Integer) (Utilities|String|ToString(Object) _array_element_2)))
        (CallFunction|ToggleFloorTile true true _array_element_2))))
  (Utilities|Array|Clear (Variables|Default|GetGapsLocal))
  ;[1 1 1] Randomize times and fill gaps array
  (for _array_element_4 PlatformsArry
    (if (not (Rendering|IsVisible _array_element_4))
      (if (< (Variables|Default|GetPlatformsVisible) 5)
        (bind _randomval (CallFunction|RandomToggle))
        (bind _hasenabled (CallFunction|ToggleFloorTile _randomval true _array_element_4))
        (if (not _hasenabled)
          (Utilities|Array|Add (Variables|Default|GetGapsLocal) (Math|Conversions|ToFloat(Integer) (Utilities|String|ToString(Object) _array_element_4)) :!label _label))
        (else
          (goto _label))))))

(fn ToggleFloorTile
  (params (Enable :type Boolean) (IncrementPlatformsVisible :type Boolean) (Tile :type Scene%20Component%20Object%20Reference))
  (Rendering|SetVisibility Tile Enable false)
  (if Enable
    (bind _asprimitive_component (Utilities|Casting|CastToPrimitiveComponent Tile)
      (:then
        (Collision|SetCollisionEnabled _asprimitive_component "QueryAndPhysics")
        (if IncrementPlatformsVisible
          (Variables|Default|SetPlatformsVisible (+ (Variables|Default|GetPlatformsVisible) 1)))
        (return Enable false))
      (:CastFailed
        _))
    (else
      (bind _asprimitive_component_2 (Utilities|Casting|CastToPrimitiveComponent Tile)
        (:then
          (Collision|SetCollisionEnabled _asprimitive_component_2 "NoCollision")
          (return Enable false))
        (:CastFailed
          _))))
  (return false true))

(fn RandomToggle
  (return (> (Math|Random|RandomFloatinRange 0.0 1.0) 0.5)))