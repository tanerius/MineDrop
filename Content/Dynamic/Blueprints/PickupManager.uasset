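; PickupManager randomly places pickups, including what is labeled gold, at socket points on a calling actor's meshes.
; After a short delay, SpawnPickups collects PickupSocket locations from the caller's visible static mesh children, passes them to RandomizePickup, then clears the list.
; RandomizePickup fills most locations with one of two child actor variants, sometimes adding gold at the same spot, positioned by offset from the manager's root.
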(event Custom|SpawnPickups
  (params (Caller :type Actor%20Object%20Reference))
  (bind _possiblelocations (Variables|Default|GetPossibleLocations))
  (Utilities|FlowControl|Delay 0.2)
  (for _array_element (Components|GetChildrenComponents (VehicleSound|GetRootComponent Caller) false)
    (bind _asstatic_mesh_component (Utilities|Casting|CastToStaticMeshComponent _array_element))
    (if (Rendering|IsVisible _asstatic_mesh_component)
      (if (Transformation|DoesSocketExist _asstatic_mesh_component "PickupSocket")
        (Utilities|Array|Add (Variables|Default|GetPossibleLocations) (Transformation|GetSocketLocation _asstatic_mesh_component "PickupSocket")))))
  (CallFunction|RandomizePickup _possiblelocations)
  (Utilities|Array|Clear _possiblelocations))

(fn ConstructionScript)

(fn RandomizePickup
  (params (Locations :type Array%20of%20Vectors))
  (for _array_element Locations
    ;[1 1 1] Dali da crtame prepreka?
    (if (< (Math|Random|RandomFloatinRange 0.0 1.0) 0.8)
      ;[1 1 1] Kakov pickup?
      (if (< (Math|Random|RandomFloatinRange 0.0 1.0) 0.5)
        (AddComponent|AddChildActorComponent false (Math|Transform|MakeTransform (- _array_element (Transformation|GetSocketLocation (VehicleSound|GetRootComponent) "None"))))
        (else
          (AddComponent|AddChildActorComponent false (Math|Transform|MakeTransform (- _array_element (Transformation|GetSocketLocation (VehicleSound|GetRootComponent) "None"))))))
      ;[1 1 1] Gold
      (if (< (Math|Random|RandomFloatinRange 0.0 1.0) 0.5)
        (AddComponent|AddChildActorComponent false (Math|Transform|MakeTransform (- _array_element (Transformation|GetSocketLocation (VehicleSound|GetRootComponent) "None"))))))))