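; JimHUD is the game's HUD, drawing the main menu, the in-game score and the game-over scoreboard.
; DrawHUD picks a state from two booleans and draws atlas regions of one UI texture, centered horizontally on screen width, with hitboxes over the buttons.
; Button clicks play a sound and call the cached JimGame game mode to start play or, after a short delay, reset.
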(event Custom|DrawScore
  ;[1 1 1] Draw score mechanic
  (if (Variables|Default|GetDrawGameOverMenu)
    ;;[1 1 1] End game score
    (HUD|DrawText (Utilities|String|ToString(Integer) (Variables|Default|GetCurrentScore)) "(R=1.000000,G=0.985380,B=0.810801,A=1.000000)" (- (* (Variables|Default|GetResX) 0.5) 2e+01) 138.0 "/Game/Static/DontDropJimAssets/JimFont.JimFont" 1.0 false)
    (HUD|DrawText (Utilities|String|ToString(Integer) (Variables|/Game/Dynamic/Blueprints/JimGame.JimGame_C|GetHighScore (Variables|Default|GetJimGameStore))) "(R=1.000000,G=0.985380,B=0.810801,A=1.000000)" (- (* (Variables|Default|GetResX) 0.5) 2e+01) 2e+02 "/Game/Static/DontDropJimAssets/JimFont.JimFont" 1.0 false)
    (else
      ;;[1 1 1] In game real time score
      (HUD|DrawText "Score: " "(R=1.000000,G=0.985380,B=0.810801,A=1.000000)" (- (* (Variables|Default|GetResX) 0.5) 1.2e+02) 0.0 "/Game/Static/DontDropJimAssets/JimFont.JimFont" 1.0 false)
      (HUD|DrawText (Utilities|String|ToString(Integer) (Variables|Default|GetCurrentScore)) "(R=1.000000,G=0.985380,B=0.810801,A=1.000000)" (- (* (Variables|Default|GetResX) 0.5) 0.9) 0.0 "/Game/Static/DontDropJimAssets/JimFont.JimFont" 1.0 false))))

(event EventDrawHUD
  (params (SizeX :type Integer) (SizeY :type Integer))
  (Variables|Default|SetResX SizeX)
  (Variables|Default|SetResY SizeY)
  (if (Variables|Default|GetDrawGameOverMenu)
    ;[1 1 1] End game reset texture and hitbox
    (Canvas|DrawTexture (Variables|Default|GetUITexture) (- (* (Variables|Default|GetResX) 0.5) (* (Variables|Default|GetResetSizeX) 0.5)) (Variables|Default|GetResetPosY) (Variables|Default|GetResetSizeX) (Variables|Default|GetResetSizeY) 0.604 0.012 0.19 0.197 "(R=1.000000,G=1.000000,B=1.000000,A=1.000000)")
    (Class|HUD|AddHitBox (Math|Vector2D|MakeVector2D (- (* (Variables|Default|GetResX) 0.5) (* (Variables|Default|GetResetSizeX) 0.5)) (Variables|Default|GetResetPosY)) (Math|Vector2D|MakeVector2D (Variables|Default|GetResetSizeX) (Variables|Default|GetResetSizeY)) (Variables|Default|GetResetHitBox) false)
    ;[1 1 1] End game scoreboard
    (Canvas|DrawTexture (Variables|Default|GetUITexture) (- (* (Variables|Default|GetResX) 0.5) (* (Variables|Default|GetScoreSizeX) 0.5)) (Variables|Default|GetResetSizeY) (Variables|Default|GetScoreSizeX) (Variables|Default|GetScoreSizeY) 0.222 0.389 0.565 0.23 "(R=1.000000,G=1.000000,B=1.000000,A=1.000000)" "BLEND_Masked")
    (CallFunction|DrawScore)
    (elif (Variables|Default|GetDrawGameMenu)
      ;[1 1 1] Main Menu hud + hitboxes
      (Canvas|DrawTexture (Variables|Default|GetUITexture) (- (* (Variables|Default|GetResX) 0.5) (* (Variables|Default|GetBtnPlaySizeX) 0.5)) (Variables|Default|GetBtnPlayPosY) (Variables|Default|GetBtnPlaySizeX) (Variables|Default|GetBtnPlaySizeY) 0.0147 0.238 0.2 0.197 "(R=1.000000,G=1.000000,B=1.000000,A=1.000000)")
      (Class|HUD|AddHitBox (Math|Vector2D|MakeVector2D (- (* (Variables|Default|GetResX) 0.5) (* (Variables|Default|GetBtnPlaySizeX) 0.5)) (Variables|Default|GetBtnPlayPosY)) (Math|Vector2D|MakeVector2D (Variables|Default|GetBtnPlaySizeX) (Variables|Default|GetBtnPlaySizeY)) (Variables|Default|GetPlayHitBox) false)
      (Canvas|DrawTexture (Variables|Default|GetUITexture) (- (* (Variables|Default|GetResX) 0.5) (* (Variables|Default|GetLogoSizeX) 0.5)) (Variables|Default|GetLogoPosY) (Variables|Default|GetLogoSizeX) (Variables|Default|GetLogoSizeY) 0.006 0.003 0.572 0.226 "(R=1.000000,G=1.000000,B=1.000000,A=1.000000)")
      (else
        (CallFunction|DrawScore)))))

(event EventHitBoxClick
  (params (BoxName :type Name))
  (bind _btnclick (Variables|Default|GetBtnClick))
  (bind _jimgamestore (Variables|Default|GetJimGameStore))
  ;[1 1 1] Hitbox event handlers
  (if (Utilities|Name|Equal(Name) BoxName (Variables|Default|GetPlayHitBox))
    (Variables|Default|SetDrawGameMenu false)
    (Audio|Components|Audio|Play _btnclick 0.0)
    (Variables|/Game/Dynamic/Blueprints/JimGame.JimGame_C|SetCanMoveLevelItems _jimgamestore true)
    (Variables|/Game/Dynamic/Blueprints/JimGame.JimGame_C|SetCanMovePlayer _jimgamestore true)
    (Default|StartGameCustom _jimgamestore)
    (elif (Utilities|Name|Equal(Name) BoxName (Variables|Default|GetResetHitBox))
      (Audio|Components|Audio|Play _btnclick 0.0)
      (Utilities|FlowControl|Delay 0.75)
      (Default|ResetGame _jimgamestore))))

(event EventBeginPlay
  (bind _asjim_game (Utilities|Casting|CastToJimGame (Game|GetGameMode)))
  (Variables|Default|SetJimGameStore _asjim_game))

(fn ConstructionScript)