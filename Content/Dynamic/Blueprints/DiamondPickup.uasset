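; DiamondPickup is a collectible that spins and bobs in place and awards 500 score when a JimCharacter overlaps it.
; Tick adds relative yaw and a sine-driven vertical offset from a wrapping angle counter, with no delta-time scaling.
; On overlap, a DoOnce sets PendingDestruction to halt the motion, adds to the score on the JimGame game mode cached at BeginPlay, plays its PickupSuccess, then destroys the actor after a short delay.
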(event EventTick
  (params (DeltaSeconds :type Float%20%28single-precision%29))
  (bind _self self)
  (bind _returnvalue (VehicleSound|GetRootComponent _self))
  ;[1 1 1] Gold ingot rotation
  (if (not (Variables|Default|GetPendingDestruction))
    (Transformation|AddRelativeRotation _returnvalue (Math|Rotator|MakeRotator 0.0 0.0 (+ (Variables|Default|GetStartingRotation) 5.0)) false false)
    ;[1 1 1] Gold ingot bounce
    (if (>= (Variables|Default|GetZMovVal) 355.0)
      (Variables|Default|SetZMovVal 0.0))
    (bind _output_get (Variables|Default|SetZMovVal (+ (Variables|Default|GetZMovVal) 8.0)))
    (bind _output_get_2 (Variables|Default|SetStaringMovement (Math|Vector|MakeVector 0.0 0.0 (Math|Trig|Sin(Degrees) _output_get))))
    (Transformation|AddRelativeLocation _returnvalue _output_get_2 false false)))

(event Collision|EventActorBeginOverlap
  (params (OtherActor :type Actor%20Object%20Reference))
  (bind _gamestore (Variables|Default|GetGameStore))
  ;[1 1 1] Collision handling
  (Utilities|Casting|CastToJimCharacter OtherActor)
  (Utilities|FlowControl|DoOnce false
    (:Completed
      (Variables|Default|SetPendingDestruction true)
      (Variables|/Game/Dynamic/Blueprints/JimGame.JimGame_C|SetScore _gamestore (+ (Variables|/Game/Dynamic/Blueprints/JimGame.JimGame_C|GetScore _gamestore) 500))
      (Audio|Components|Audio|Play (Variables|/Game/Dynamic/Blueprints/JimGame.JimGame_C|GetPickupSuccess _gamestore) 0.0)
      (Utilities|FlowControl|Delay 0.1)
      (Actor|DestroyActor))))

(event EventBeginPlay
  ;[1 1 1] Setup class
  (Variables|Default|SetStaringMovement "0, 0, 0")
  (Variables|Default|SetZMovVal 0.0)
  (bind _asjim_game (Utilities|Casting|CastToJimGame (Game|GetGameMode)))
  (Variables|Default|SetGameStore _asjim_game)
  (Variables|Default|SetPendingDestruction false))

(fn ConstructionScript)