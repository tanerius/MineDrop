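; TopPlatformSet is a set of platform components in two numbered groups that builds a partly random layout on BeginPlay.
; The first group is fixed at half shown and half hidden, with collision matching visibility.
; In the second, 2.4 always shows and the others have even odds of appearing, capped at five visible so one gap remains.
; Failed rolls are recorded by name in Gaps, but platforms skipped after the cap are not.
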(event EventBeginPlay
  (bind _2_4 (Variables|PlatformMeshes|Get2.4))
  (bind _2_2 (Variables|PlatformMeshes|Get2.2))
  (bind _1_1 (Variables|PlatformMeshes|Get1.1))
  (bind _1_4 (Variables|PlatformMeshes|Get1.4))
  (Rendering|SetVisibility _1_1 true false)
  (Collision|SetCollisionEnabled _1_1 "QueryAndPhysics")
  (Rendering|SetVisibility _1_4 false false)
  (Collision|SetCollisionEnabled _1_4 "NoCollision")
  (Rendering|SetVisibility _2_4 true false)
  (Collision|SetCollisionEnabled _2_4 "QueryAndPhysics")
  (Variables|Default|SetPlatformsVisible 1)
  (Rendering|SetVisibility _2_2 false false)
  (Collision|SetCollisionEnabled _2_2 "NoCollision")
  (for _array_element (Utilities|Array|MakeArray (Variables|PlatformMeshes|Get2.1) (Variables|PlatformMeshes|Get2.2) (Variables|PlatformMeshes|Get2.3) (Variables|PlatformMeshes|Get2.4) (Variables|PlatformMeshes|Get2.5) (Variables|PlatformMeshes|Get2.6))
    (if (not (Rendering|IsVisible _array_element))
      (if (< (Variables|Default|GetPlatformsVisible) 5)
        (Rendering|SetVisibility _array_element (> (Math|Random|RandomFloatinRange 0.0 1.0) 0.5) false)
        (if (Rendering|IsVisible _array_element)
          (Collision|SetCollisionEnabled _array_element "QueryAndPhysics")
          (Variables|Default|SetPlatformsVisible (+ (Variables|Default|GetPlatformsVisible) 1))
          (else
            (Utilities|Array|Add (Variables|Default|GetGaps) (Utilities|String|ToString(Object) _array_element))))))))

(fn ConstructionScript)