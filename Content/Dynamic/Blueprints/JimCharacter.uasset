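; JimCharacter is a player character that walks automatically along the world Y axis and turns around when clicked.
; Tick adds movement input in the current direction, while each click flip-flops the direction flag and actor rotation.
; Both walking and turning depend on the CanMovePlayer flag in the JimGame game mode.
; BeginPlay caches that game mode, sets the starting rotation, then runs a Delay loop that raises max walk speed up to a threshold.
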(event MouseInput|EventActorOnClicked
  (params (ButtonPressed :type Key%20Structure :default "AnyKey"))
  ;[1 1 1] Turning
  (if (Variables|/Game/Dynamic/Blueprints/JimGame.JimGame_C|GetCanMovePlayer (Variables|Default|GetJimGameStore))
    (bind _isa (Utilities|FlowControl|FlipFlop)
      (:A
        (Variables|Default|SetWalkDirectionInv _isa)
        (Transformation|SetActorRotation (Variables|Default|GetLeftDirectionPawn)))
      (:B
        (Variables|Default|SetWalkDirectionInv _isa)
        (Transformation|SetActorRotation (Variables|Default|GetRightDirectionPawn))))))

(event EventBeginPlay
  ;[1 1 1] Set initial player rotation
  (bind _asjim_game (Utilities|Casting|CastToJimGame (Game|GetGameMode)))
  (Variables|Default|SetJimGameStore _asjim_game)
  (Transformation|SetActorRotation "0,-90.000000, 0")
  ;[1 1 1] Speed Increase Mechanic
  (if (< (Variables|Default|GetSpeed) 375.0) :!label _label
    (Variables|Default|SetSpeed (+ (Variables|Default|GetSpeedIncrease) (Variables|Default|GetSpeed)))
    (Variables|/Script/Engine.CharacterMovementComponent|SetMaxWalkSpeed (Variables|Character|GetCharacterMovement) (Variables|Default|GetSpeed))
    (Utilities|FlowControl|Delay (Variables|Default|GetRateOfIncrease))
    (goto _label)))

(event EventTick
  (params (DeltaSeconds :type Float%20%28single-precision%29))
  (bind _returnvalue (Transformation|GetActorLocation))
  ;[1 1 1] Walking
  (if (Variables|/Game/Dynamic/Blueprints/JimGame.JimGame_C|GetCanMovePlayer (Variables|Default|GetJimGameStore))
    (if (Variables|Default|GetWalkDirectionInv)
      (Pawn|Input|AddMovementInput (Math|Transform|TransformDirection (Math|Conversions|ToTransform(Vector) _returnvalue) "0,1.000000, 0") 1.0 false)
      (else
        (Pawn|Input|AddMovementInput (Math|Transform|TransformDirection (Math|Conversions|ToTransform(Vector) _returnvalue) "0,-1.000000, 0") 1.0 false)))))

(fn ConstructionScript)