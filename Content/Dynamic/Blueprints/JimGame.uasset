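; JimGame is the game logic Blueprint for Jim, handling the running score, saved high score, player death and restarts.
; On BeginPlay it loads the high score from the "Jim" save slot and caches the JimHUD reference.
; StartGameCustom runs a Delay loop that raises Score and pushes it to the HUD while CanMovePlayer is true.
; PlayerDies saves any new high score, stops movement and shows the game-over menu.
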(event Custom|ResetGame
  ;[1 1 1] Reset game mechanic
  (Class|GameMode|RestartGame))

(event Custom|StartGameCustom
  ;[1 1 1] Update score mechanic
  (if (Variables|Default|GetCanMovePlayer) :!label _label
    (bind _output_get (Variables|Default|SetScore (+ (Variables|Default|GetScore) 5)))
    (Utilities|FlowControl|Delay 0.2)
    (Variables|/Game/Dynamic/Blueprints/JimHUD.JimHUD_C|SetCurrentScore (Variables|Default|GetJimHUDRef) _output_get)
    (goto _label)))

(event Custom|PlayerDies
  ;[1 1 1] When player dies
  (CallFunction|SaveGame)
  (Utilities|FlowControl|Delay 0.05)
  (Variables|Default|SetCanMoveLevelItems false)
  (Variables|Default|SetCanMovePlayer false)
  (Variables|/Game/Dynamic/Blueprints/JimHUD.JimHUD_C|SetDrawGameOverMenu (Variables|Default|GetJimHUDRef) true))

(event Custom|SaveGame
  (bind _score (Variables|Default|GetScore))
  ;[1 1 1] Save game logic
  (if (> (Variables|Default|GetScore) (Variables|Default|GetHighScore))
    (Variables|Default|SetHighScore (Variables|Default|GetScore))
    (bind _returnvalue (SaveGame|DoesSaveGameExist "Jim"))
    (if _returnvalue
      (Variables|/Game/Dynamic/Blueprints/JimSaveGame.JimSaveGame_C|SetSavedHighScore (Variables|Default|GetSaveGameObj) _score)
      (SaveGame|SaveGametoSlot (Variables|Default|GetSaveGameObj) "Jim")
      (else
        (bind _returnvalue_2 (SaveGame|CreateSaveGameObject "/Game/Dynamic/Blueprints/JimSaveGame.JimSaveGame_C"))
        (bind _output_get (Variables|Default|SetSaveGameObj _returnvalue_2))
        (Variables|/Game/Dynamic/Blueprints/JimSaveGame.JimSaveGame_C|SetSavedHighScore _output_get _score)
        (SaveGame|SaveGametoSlot (Variables|Default|GetSaveGameObj) "Jim")))))

(event EventBeginPlay
  ;[1 1 1] Load saved game
  (bind _returnvalue (SaveGame|DoesSaveGameExist "Jim"))
  (if _returnvalue
    (bind _returnvalue_2 (SaveGame|LoadGamefromSlot "Jim"))
    (bind _asjim_save_game (Utilities|Casting|CastToJimSaveGame _returnvalue_2))
    (bind _output_get (Variables|Default|SetSaveGameObj _asjim_save_game))
    (Variables|Default|SetHighScore (Variables|/Game/Dynamic/Blueprints/JimSaveGame.JimSaveGame_C|GetSavedHighScore _output_get))
    (else
      (Variables|Default|SetHighScore 0)))
  ;[1 1 1] Get reference to hud
  (bind _asjim_hud (Utilities|Casting|CastToJimHUD (HUD|GetHUD (Game|GetPlayerController 0))))
  (Variables|Default|SetJimHUDRef _asjim_hud))

(fn ConstructionScript)